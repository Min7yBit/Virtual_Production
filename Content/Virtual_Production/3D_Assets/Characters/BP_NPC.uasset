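; NPC character Blueprint for a virtual production project that plays scene animations on demand from input.
; On BeginPlay it enables input from player controller 0, so Scene 1 to 4 input actions each trigger a one-shot PlayAnimation on the skeletal mesh.
; Scene 2 has its own animation, while Scenes 3 and 4 reuse the Scene 1 Xsens mocap take.
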(event EventBeginPlay
  (Input|EnableInput (Game|GetPlayerController 0)))

(event Collision|EventActorBeginOverlap
  (params (OtherActor :type Actor%20Object%20Reference)))

(event EventTick
  (params (DeltaSeconds :type Float%20%28single-precision%29)))

(event Input|ActionEvents|InputActionScene1
  (params (Key :type Key%20Structure :default "None"))
  (:Pressed
    (Components|Animation|PlayAnimation (Variables|SkeletalMeshActor|GetSkeletalMeshComponent) "/Game/Virtual_Production/3D_Assets/Characters/scene_1_working_2_Anim_main_arma_001_Reference_Scene_1_and_2-Scene_1_take_4_Xsens_Animation_Laye_002.scene_1_working_2_Anim_main_arma_001_Reference_Scene_1_and_2-Scene_1_take_4_Xsens_Animation_Laye_002" false)))

(event Input|ActionEvents|InputActionScene2
  (params (Key :type Key%20Structure :default "None"))
  (:Pressed
    (Components|Animation|PlayAnimation (Variables|SkeletalMeshActor|GetSkeletalMeshComponent) "/Game/Virtual_Production/3D_Assets/Characters/scene_2/scene_2_final_Anim_main_arma_Action.scene_2_final_Anim_main_arma_Action" false)))

(event Input|ActionEvents|InputActionScene3
  (params (Key :type Key%20Structure :default "None"))
  (:Pressed
    (Components|Animation|PlayAnimation (Variables|SkeletalMeshActor|GetSkeletalMeshComponent) "/Game/Virtual_Production/3D_Assets/Characters/scene_1_working_2_Anim_main_arma_001_Reference_Scene_1_and_2-Scene_1_take_4_Xsens_Animation_Laye_002.scene_1_working_2_Anim_main_arma_001_Reference_Scene_1_and_2-Scene_1_take_4_Xsens_Animation_Laye_002" false)))

(event Input|ActionEvents|InputActionScene4
  (params (Key :type Key%20Structure :default "None"))
  (:Pressed
    (Components|Animation|PlayAnimation (Variables|SkeletalMeshActor|GetSkeletalMeshComponent) "/Game/Virtual_Production/3D_Assets/Characters/scene_1_working_2_Anim_main_arma_001_Reference_Scene_1_and_2-Scene_1_take_4_Xsens_Animation_Laye_002.scene_1_working_2_Anim_main_arma_001_Reference_Scene_1_and_2-Scene_1_take_4_Xsens_Animation_Laye_002" false)))

(fn ConstructionScript)