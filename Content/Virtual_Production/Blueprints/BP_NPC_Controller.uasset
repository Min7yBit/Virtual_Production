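; BP_NPC_Controller is a virtual production actor that triggers NPC animations per scene from player input.
; On BeginPlay it enables input from player controller 0.
; Four Scene input actions each check their matching NPC scene reference and, if valid, call PlayAnimation on it.
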(event EventBeginPlay
  (Input|EnableInput (Game|GetPlayerController 0)))

(event Input|ActionEvents|InputActionScene1
  (params (Key :type Key%20Structure :default "None"))
  (bind _npcscene1 (Variables|Default|GetNpcScene1))
  (:Pressed
    (Utilities|IsValid _npcscene1
      (:Is%20Valid
        (Default|PlayAnimation _npcscene1)))))

(event Input|ActionEvents|InputActionScene2
  (params (Key :type Key%20Structure :default "None"))
  (bind _npcscene2 (Variables|Default|GetNpcScene2))
  (:Pressed
    (Utilities|IsValid _npcscene2
      (:Is%20Valid
        (Default|PlayAnimation _npcscene2)))))

(event Input|ActionEvents|InputActionScene3
  (params (Key :type Key%20Structure :default "None"))
  (bind _npcscene3 (Variables|Default|GetNpcScene3))
  (:Pressed
    (Utilities|IsValid _npcscene3
      (:Is%20Valid
        (Default|PlayAnimation _npcscene3)))))

(event Input|ActionEvents|InputActionScene4
  (params (Key :type Key%20Structure :default "None"))
  (bind _npcscene4 (Variables|Default|GetNpcScene4))
  (:Pressed
    (Utilities|IsValid _npcscene4
      (:Is%20Valid
        (Default|PlayAnimation _npcscene4)))))

(fn ConstructionScript)