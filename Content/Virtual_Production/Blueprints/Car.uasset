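; Car is an actor in the Virtual Production content that drives straight ahead and removes itself after a countdown.
; Every tick, MoveCar offsets its location along the root component's forward vector by Speed scaled by delta time, without sweeping for collision.
; DespawnCar counts DespawnTImer down, prints the remaining time on screen, and destroys the actor once it drops below zero.
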(event EventTick
  (params (DeltaSeconds :type Float%20%28single-precision%29))
  (CallFunction|MoveCar DeltaSeconds)
  (CallFunction|DespawnCar DeltaSeconds))

(fn ConstructionScript)

(fn MoveCar
  (params (Delta%20Time :type Float%20%28single-precision%29))
  (Transformation|SetActorLocation (+ (* (* (Math|Vector|GetForwardVector (Variables|Default|GetDefaultSceneRoot)) (Variables|Default|GetSpeed)) Delta%20Time) (Transformation|GetWorldLocation (Variables|Default|GetDefaultSceneRoot))) false false))

(fn DespawnCar
  (params (Seconds :type Float%20%28single-precision%29))
  (bind _output_get (Variables|Default|SetDespawn%20TImer (- (Variables|Default|GetDespawn%20TImer) Seconds)))
  (if (< _output_get 0.0)
    (Development|PrintString "Destory Car")
    (Actor|DestroyActor)
    (else
      (Development|PrintString (Utilities|String|Append "Drespawn time" (Utilities|String|ToString(Float) _output_get))))))