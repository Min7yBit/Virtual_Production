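; Virtual production bar attachment Blueprint that switches the emissive lights on its static mesh on and off.
; BeginPlay sets the materials' Emissive scalar parameter to EmissiveValue.
; ToggleBarLights replays a timeline from the start, scaling EmissiveValue by its LightIntensity curve for both directions.
; When the timeline finishes, it snaps Emissive to zero or full based on LightsOn and flips that flag.
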(event Custom|Toggle%20Bar%20Lights
  (bind _staticmeshcomponent (Variables|Debug|GetStaticMeshComponent))
  (bind _light_intensity (Timeline|Timeline_0 PlayFromStart)
    (:Update
      (Rendering|Material|SetScalarParameterValueonMaterials (Variables|Debug|GetStaticMeshComponent) "Emissive" (* _light_intensity (Variables|Default|GetEmissiveValue))))
    (:Finished
      (if (Variables|Default|GetLightsOn)
        (Rendering|Material|SetScalarParameterValueonMaterials _staticmeshcomponent "Emissive" 0.0)
        (Variables|Default|SetLightsOn false)
        (else
          (Rendering|Material|SetScalarParameterValueonMaterials _staticmeshcomponent "Emissive" (Variables|Default|GetEmissiveValue))
          (Variables|Default|SetLightsOn true))))))

(event EventBeginPlay
  (Rendering|Material|SetScalarParameterValueonMaterials (Variables|Debug|GetStaticMeshComponent) "Emissive" (Variables|Default|GetEmissiveValue)))

(fn ConstructionScript)