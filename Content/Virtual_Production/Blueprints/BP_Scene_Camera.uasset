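; Virtual production scene camera Blueprint that makes a referenced Camera actor the first player's view target on BeginPlay and smooths its motion.
; On each Live Link update, it lerps from the last applied transform toward the CameraLocation world transform, using DeltaTime times SmoothingValue as alpha.
; The resulting location and rotation move the Camera and are stored with unit scale for the next update, easing out tracking movement.
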(event OnLiveLinkUpdated(LiveLinkComponentController)
  (params (DeltaTime :type Float%20%28single-precision%29))
  (Transformation|SetActorLocationAndRotation (Variables|Default|GetCamera) (.location (Math|Transform|Lerp(Transform) (Variables|Default|GetLast%20Transform) (Transformation|GetWorldTransform (Variables|Default|GetCamera%20Location)) (* DeltaTime (Variables|Default|GetSmoothing%20Value)))) (.rotation (Math|Transform|Lerp(Transform) (Variables|Default|GetLast%20Transform) (Transformation|GetWorldTransform (Variables|Default|GetCamera%20Location)) (* DeltaTime (Variables|Default|GetSmoothing%20Value)))))
  (Variables|Default|SetLast%20Transform (Math|Transform|MakeTransform (.location (Math|Transform|Lerp(Transform) (Variables|Default|GetLast%20Transform) (Transformation|GetWorldTransform (Variables|Default|GetCamera%20Location)) (* DeltaTime (Variables|Default|GetSmoothing%20Value)))) (.rotation (Math|Transform|Lerp(Transform) (Variables|Default|GetLast%20Transform) (Transformation|GetWorldTransform (Variables|Default|GetCamera%20Location)) (* DeltaTime (Variables|Default|GetSmoothing%20Value)))) "1,1,1")))

(event EventBeginPlay
  (Game|Player|SetViewTargetwithBlend (Game|GetPlayerController 0) (Variables|Default|GetCamera) 0.0 "VTBlend_Linear" 0.0 false))

(event Collision|EventActorBeginOverlap
  (params (OtherActor :type Actor%20Object%20Reference)))

(event EventTick
  (params (DeltaSeconds :type Float%20%28single-precision%29)))

(fn ConstructionScript)