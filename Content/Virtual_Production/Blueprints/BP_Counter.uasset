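; BP_Counter is a counter actor with emissive lights that can be toggled on and off.
; BeginPlay sets the mesh materials' Emissive scalar parameter to EmissiveValue.
; ToggleCounterLights plays a timeline that scales Emissive by a LightIntensity curve, then sets it to zero or full and flips LightsOn.
; The same curve plays from the start in both toggle directions, with only the final value differing.
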(event Custom|Toggle%20Counter%20Lights
  (bind _staticmeshcomponent (Variables|Debug|GetStaticMeshComponent))
  (bind _light_intensity (Timeline|Timeline_0 PlayFromStart)
    (:Update
      (Rendering|Material|SetScalarParameterValueonMaterials (Variables|Debug|GetStaticMeshComponent) "Emissive" (* _light_intensity (Variables|Default|GetEmissiveValue))))
    (:Finished
      (if (Variables|Components|GetLightsOn)
        (Rendering|Material|SetScalarParameterValueonMaterials _staticmeshcomponent "Emissive" 0.0)
        (Variables|Components|SetLightsOn false)
        (else
          (Rendering|Material|SetScalarParameterValueonMaterials _staticmeshcomponent "Emissive" (Variables|Default|GetEmissiveValue))
          (Variables|Components|SetLightsOn true))))))

(event EventBeginPlay
  (Rendering|Material|SetScalarParameterValueonMaterials (Variables|Debug|GetStaticMeshComponent) "Emissive" (Variables|Default|GetEmissiveValue)))

(fn ConstructionScript)