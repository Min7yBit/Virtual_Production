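; BP_Lights is a virtual production light Blueprint that toggles a point light on and off through a timeline-animated transition.
; On BeginPlay it caches the light's initial intensity and enables input from the first player controller.
; ToggleLights replays the timeline from the start in both directions, scaling the cached intensity by its curve.
; When the timeline finishes, it snaps to zero or full intensity and flips the LightsOn state.
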(event Custom|Toggle%20Lights
  (bind _pointlight (Variables|Default|GetPointLight))
  (bind _light_intensity (Timeline|Timeline_0 PlayFromStart)
    (:Update
      (Rendering|Components|Light|SetIntensity _pointlight (* _light_intensity (Variables|Components|GetInitial%20Light%20Intensity))))
    (:Finished
      (if (Variables|Components|GetLightsOn)
        (Rendering|Components|Light|SetIntensity _pointlight 0.0)
        (Variables|Components|SetLightsOn false)
        (else
          (Rendering|Components|Light|SetIntensity _pointlight (Variables|Components|GetInitial%20Light%20Intensity))
          (Variables|Components|SetLightsOn true))))))

(event EventBeginPlay
  (Variables|Components|SetInitial%20Light%20Intensity (Variables|/Script/Engine.LightComponentBase|GetIntensity (Variables|Default|GetPointLight)))
  (Input|EnableInput (Game|GetPlayerController 0)))

(fn ConstructionScript)