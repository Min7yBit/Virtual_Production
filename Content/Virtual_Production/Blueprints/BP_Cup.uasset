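; BP_Cup is a cup actor that can be picked up and released by a Test_Blueprint character's left hand.
; Overlap with that actor sets a contact flag and enables player input on the cup; ending overlap clears the flag.
; The G key attaches the cup to the LeftHandSocket while in contact, or detaches it in place if held.
; The GrabCup input action only prints a debug message.
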(event Collision|EventActorBeginOverlap
  (params (OtherActor :type Actor%20Object%20Reference))
  (bind _astest_blueprint (Utilities|Casting|CastToTest_Blueprint OtherActor))
  (Development|PrintString "hit hand")
  (Variables|Default|SetinContactWithCup true)
  (Input|EnableInput (Game|GetPlayerController 0)))

(event Collision|EventActorEndOverlap
  (params (OtherActor :type Actor%20Object%20Reference))
  (Utilities|Casting|CastToTest_Blueprint OtherActor)
  (Development|PrintString "Let Hand")
  (Variables|Default|SetinContactWithCup false))

(event Input|ActionEvents|InputActionGrabCup
  (params (Key :type Key%20Structure :default "None"))
  (:Pressed
    (Development|PrintString "Pressed Grabbed cup")))

(event Input|KeyboardEvents|G
  (params (Key :type Key%20Structure :default "None"))
  (:Pressed
    (if (Variables|Default|GetisHoldingCup)
      (Transformation|DetachFromComponent (Variables|Default|GetDefaultSceneRoot) "KeepWorld" "KeepWorld" "KeepWorld" true)
      (Variables|Default|SetisHoldingCup false)
      (elif (Variables|Default|GetinContactWithCup)
        (Transformation|AttachComponentToComponent (Variables|/Script/Engine.SkeletalMeshActor|GetSkeletalMeshComponent (stale Collision|EventActorBeginOverlap _astest_blueprint)) "LeftHandSocket" "SnapToTarget" "SnapToTarget" "KeepWorld" false)
        (Variables|Default|SetisHoldingCup true)))))

(fn ConstructionScript)