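; Controller actor for virtual production that toggles a set of spark effect actors on and off with an input action.
; On BeginPlay it enables input from player controller 0 and deactivates the particle component of every referenced spark actor.
; The Toggle Sparks action calls a function that loops over the Sparks array and tells each actor to toggle itself.
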(event EventBeginPlay
  (Input|EnableInput (Game|GetPlayerController 0))
  (for _array_element (Variables|Default|GetSparks)
    (Components|Activation|Deactivate (Variables|/Game/Virtual_Production/Blueprints/BP_Sparks.BP_Sparks_C|GetSparks_Particle _array_element))))

(event Input|ActionEvents|InputActionToggleSparks
  (params (Key :type Key%20Structure :default "None"))
  (:Pressed
    (CallFunction|ToggleSparks)))

(fn ConstructionScript)

(fn ToggleSparks
  (for _array_element (Variables|Default|GetSparks)
    (Default|ToggleSparks _array_element)))