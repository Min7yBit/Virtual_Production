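; BP_Lights_BarLight is a virtual production bar light whose point light toggles on and off with a flicker.
; BeginPlay caches the starting intensity and enables player input.
; ToggleLights plays the LightFlicker timeline to scale that intensity, then flips LightsOn and sets zero or full brightness.
; TurnLightsOn and TurnLightsOff are unfinished stubs, the latter holding an empty loop and disconnected random-flicker nodes.
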(event Custom|Toggle%20Lights
  (bind _pointlight (Variables|Default|GetPointLight))
  (bind _light_intensity (Timeline|Light%20Flicker PlayFromStart)
    (:Update
      (Rendering|Components|Light|SetIntensity _pointlight (* _light_intensity (Variables|Default|GetInitial%20Light%20Intensity))))
    (:Finished
      (if (Variables|Default|GetLightsOn)
        (Rendering|Components|Light|SetIntensity _pointlight 0.0)
        (Variables|Default|SetLightsOn false)
        (else
          (Rendering|Components|Light|SetIntensity _pointlight (Variables|Default|GetInitial%20Light%20Intensity))
          (Variables|Default|SetLightsOn true))))))

(event EventBeginPlay
  (Variables|Default|SetInitial%20Light%20Intensity (Variables|/Script/Engine.LightComponentBase|GetIntensity (Variables|Default|GetPointLight)))
  (Input|EnableInput (Game|GetPlayerController 0)))

(fn ConstructionScript)

(fn TurnLightson
  (return true))

(fn TurnLightsOff
  (for _index (range 0 15)
    _))